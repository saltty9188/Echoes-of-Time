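; Enemy actor that chases the player across past, present and future tile maps, damaging them on overlap.
; Each tick it follows an A* path, using a sorted-array priority queue, rerouting when the player's tile changes and homing directly when close.
; It teleports beside the camera bounds when too far, on time travel or on respawn.
; Death spawns an explosion and random pickup, then it respawns after a delay; player death also respawns it.
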(event OnComponentBeginOverlap(Box)
  (params (OverlappedComponent :type Primitive%20Component%20Object%20Reference) (OtherActor :type Actor%20Object%20Reference) (OtherComp :type Primitive%20Component%20Object%20Reference) (OtherBodyIndex :type Integer) (bFromSweep :type Boolean) (SweepResult :type Hit%20Result%20Structure%20%28by%20ref%29))
  ;[1 1 1] Damage Player
  (bind _asplayer_character (Utilities|Casting|CastToPlayerCharacter OtherActor))
  (Default|TakeDamage _asplayer_character 2e+01)
  (Collision|SetCollisionEnabled (Variables|Default|GetRenderComponent) "NoCollision"))

(event OnComponentEndOverlap(Box)
  (params (OverlappedComponent :type Primitive%20Component%20Object%20Reference) (OtherActor :type Actor%20Object%20Reference) (OtherComp :type Primitive%20Component%20Object%20Reference) (OtherBodyIndex :type Integer))
  (Utilities|Casting|CastToPlayerCharacter OtherActor)
  (Collision|SetCollisionEnabled (Variables|Default|GetRenderComponent) "QueryOnly"))

(event Custom|OnTimeTravel
  (params (NewZOffset :type Float%20%28single-precision%29))
  (CallFunction|ChangeMaps NewZOffset)
  (Variables|Default|SetTrackingPlayer true))

(event Custom|DamageFlash
  (bind _paperflipbook (Variables|Default|GetPaperFlipbook))
  ;[1 1 1] Damage Flash
  (Utilities|ForLoopwithDelay 0 1 0.1
    (:Loop%20Body
      (Rendering|SetVisibility _paperflipbook (not (Rendering|IsVisible _paperflipbook)) false))
    (:Completed
      (Rendering|SetVisibility (Variables|Default|GetPaperFlipbook) true false))))

(event Custom|RespawnEvent
  (CallFunction|Respawn))

(event EventBeginPlay
  (bind _asplayer_character (Utilities|Casting|CastToPlayerCharacter (Game|Player|GetPlayerPawn 0)))
  (EventDispatchers|BindEventtoTimeTravelEventDispatcher _asplayer_character (delegate Custom|OnTimeTravel))
  (EventDispatchers|BindEventtoDeathEventDispatcher _asplayer_character (delegate Custom|RespawnEvent)))

(event EventTick
  (params (DeltaSeconds :type Float%20%28single-precision%29))
  (bind _returnvalue (Game|Player|GetPlayerPawn 0))
  (bind _returnvalue_2 (Transformation|GetActorLocation))
  (bind _returnvalue_3 (Transformation|GetActorLocation _returnvalue))
  (bind (_x _y _z) (Math|Vector|BreakVector _returnvalue_2))
  (bind (_x_2 _y_2 _z_2) (Math|Vector|BreakVector _returnvalue_3))
  ;[1 1 1] Respawn after 10 seconds
  (if (> (Variables|Default|GetRespawnTimer) 0.0)
    (bind _output_get (Variables|Default|SetRespawnTimer (- (Variables|Default|GetRespawnTimer) DeltaSeconds)))
    (if (<= _output_get 0.0)
      (CallFunction|Respawn)))
  ;[1 1 1] Teleport closer if too far off screen
  (if (Variables|Default|GetTrackingPlayer)
    (bind _output_get_2 (Variables|Default|SetDistFromPlayer (Math|Vector|Distance(Vector) (Transformation|GetActorLocation) (Transformation|GetActorLocation (Game|Player|GetPlayerPawn 0)))))
    (if (> _output_get_2 7e+02)
      (CallFunction|TeleportOffscreen)
      (bind _player (CallFunction|ASTar :!label _label))
      (Variables|Default|SetLastKnownGoal _player)
      (else
        ;[1 1 1] Check if Reroute needed
        (bind _tile (Default|GetTile (Variables|Default|GetCurrentMap) (Math|Vector|MakeVector _x_2 _y_2 (- _z_2 (Variables|Default|GetZOffset)))))
        (bind _equal (CallFunction|AreTilesEqual _tile (Variables|Default|GetLastKnownGoal)))
        (if _equal
          _
          (else
            (goto _label)))))
    (bind _tile_2 (Default|GetTile (Variables|Default|GetCurrentMap) (Math|Vector|MakeVector _x _y (- _z (Variables|Default|GetZOffset)))))
    (Variables|Default|SetCurrentTile _tile_2)
    ;[1 1 1] If in same large tile as the target move directly towards the target
    (Variables|Default|SetLowestCostTile (Variables|Default|GetLastKnownGoal))
    (if (< (Variables|Default|GetDistFromPlayer) 64.0)
      (CallFunction|MoveinDirection (Math|Vector|GetUnitDirection(Vector) (Transformation|GetActorLocation) (Transformation|GetActorLocation (Game|Player|GetPlayerPawn 0))) DeltaSeconds)
      (else
        (Variables|Default|SetIs%20Neighbour false)
        (while (not (Variables|Default|GetIs%20Neighbour))
          ;[1 1 1] Backpropogate to the next tile
          (bind _output_get_3 (Variables|Default|SetLowestCostTile (Utilities|Array|Get(acopy) (Variables|/Game/Blueprints/AI/AITileMap.AITileMap_C|GetMapTiles (Variables|Default|GetCurrentMap)) (.Value (Utilities|Map|Find (Variables|Default|GetCameFrom) (.index (Variables|Default|GetLowestCostTile)))))))
          (Variables|Default|SetIs%20Neighbour (Utilities|Array|ContainsItem (.neighbourindices (Variables|Default|GetCurrentTile)) (.index _output_get_3))))
        ;[1 1 1] Move towards the lowest cost neighbour
        (bind _returnvalue_4 (Default|GetTileWorldPosition (Variables|Default|GetCurrentMap) (.X (Utilities|Struct|BreakAITile (Variables|Default|GetLowestCostTile))) (.Y (Utilities|Struct|BreakAITile (Variables|Default|GetLowestCostTile)))))
        (CallFunction|MoveinDirection (Math|Vector|GetUnitDirection(Vector) (Transformation|GetActorLocation) _returnvalue_4) DeltaSeconds)))))

(fn ConstructionScript)

(fn Heuristic
  (params (NextTile :type AI%20Tile%20Structure) (GoalTile :type AI%20Tile%20Structure))
  (bind (_canpass _x _y) (Utilities|Struct|BreakAITile NextTile))
  (bind (_canpass_2 _x_2 _y_2) (Utilities|Struct|BreakAITile GoalTile))
  (return (+ (Math|Integer|Absolute(Integer) (- _x _x_2)) (Math|Integer|Absolute(Integer) (- _y _y_2)))))

(fn ConverttoGridCoordinates
  (params (WorldPosition :type Vector))
  (bind (_x _y _z) (Math|Vector|BreakVector WorldPosition))
  (return (Math|Float|Truncate (/ _x 16.0)) (Math|Float|Truncate (/ (- _z (Variables|Default|GetZOffset)) -16.0))))

(fn ASTar
  (bind _returnvalue (Transformation|GetActorLocation))
  (bind _returnvalue_2 (Game|Player|GetPlayerPawn 0))
  (bind _frontier (LocalVariables|GetFrontier))
  (bind _returnvalue_3 (Transformation|GetActorLocation _returnvalue_2))
  (Utilities|IsValid (Variables|Default|GetCurrentMap)
    (:Is%20Valid
      _)
    (:Is%20Not%20Valid
      (Variables|Default|SetCurrentMap (Variables|Default|GetPresentMap))))
  (Utilities|Map|Clear (Variables|Default|GetCostSoFar))
  (Utilities|Map|Clear (Variables|Default|GetCameFrom))
  (bind _tile (Default|GetTile (Variables|Default|GetCurrentMap) (Math|Vector|MakeVector (.x _returnvalue) 0.0 (- (.z _returnvalue) (Variables|Default|GetZOffset)))))
  (LocalVariables|SetStart _tile)
  (bind _tile_2 (Default|GetTile (Variables|Default|GetCurrentMap) (Math|Vector|MakeVector (.x _returnvalue_3) 0.0 (- (.z _returnvalue_3) (Variables|Default|GetZOffset)))))
  (LocalVariables|SetGoal _tile_2)
  (Utilities|Array|Add (LocalVariables|GetFrontier) (Utilities|Struct|MakePrioritizedAITile (LocalVariables|GetStart) 0.0))
  (Utilities|Map|Add (Variables|Default|GetCameFrom) (.Index (Utilities|Struct|BreakAITile (LocalVariables|GetStart))) (.Index (Utilities|Struct|BreakAITile (LocalVariables|GetStart))))
  (Utilities|Map|Add (Variables|Default|GetCostSoFar) (.Index (Utilities|Struct|BreakAITile (LocalVariables|GetStart))) 0.0)
  (while (> (Utilities|Array|Length (LocalVariables|GetFrontier)) 0)
    (bind _output (CallFunction|QueuePop (LocalVariables|GetFrontier)))
    (bind _output_get (LocalVariables|SetCurrent (.tile _output)))
    (bind _equal (CallFunction|AreTilesEqual _output_get (LocalVariables|GetGoal)))
    (if _equal
      ;[1 1 1] Break early if found goal
      (Utilities|Array|Resize (LocalVariables|GetFrontier) 0)
      (return (LocalVariables|GetGoal))
      (else
        (for _array_element (.NeighbourIndices (Utilities|Struct|BreakAITile _output_get))
          (bind _output_get_2 (LocalVariables|SetNext (Utilities|Array|Get(acopy) (Variables|/Game/Blueprints/AI/AITileMap.AITileMap_C|GetMapTiles (Variables|Default|GetCurrentMap)) _array_element)))
          ;[1 1 1] Get the new cost to the next tile from the current one
          (bind _cost (CallFunction|MovementCost (LocalVariables|GetCurrent) _output_get_2))
          (bind _output_get_3 (LocalVariables|SetNewCost (+ _cost (.Value (Utilities|Map|Find (Variables|Default|GetCostSoFar) (.Index (Utilities|Struct|BreakAITile (LocalVariables|GetCurrent))))))))
          (if (not (.ReturnValue (Utilities|Map|Find (Variables|Default|GetCostSoFar) (.index (LocalVariables|GetNext)))))
            ;[1 1 1] Update the cost if its newly discovered or lower than the previous
            (Utilities|Map|Add (Variables|Default|GetCostSoFar) (.index (LocalVariables|GetNext)) (LocalVariables|GetNewCost) :!label _label)
            (bind _returnvalue_4 (CallFunction|Heuristic (LocalVariables|GetNext) (LocalVariables|GetGoal)))
            ;[1 1 1] Hacky "Priority Queue"
            (Utilities|Array|Add _frontier (Utilities|Struct|MakePrioritizedAITile (LocalVariables|GetNext) (+ (Math|Conversions|ToFloat(Integer) _returnvalue_4) (LocalVariables|GetNewCost))))
            (Class|MyBlueprintFunctionLibrary|TilePrioritySort _frontier)
            ;[1 1 1] Record what the previous tile was to get this cost
            (Utilities|Map|Add (Variables|Default|GetCameFrom) (.index (LocalVariables|GetNext)) (.index (LocalVariables|GetCurrent)))
            (elif (< _output_get_3 (.Value (Utilities|Map|Find (Variables|Default|GetCostSoFar) (.index (LocalVariables|GetNext)))))
              (goto _label))))))))

(fn QueuePop
  (params (NewParam :type Array%20of%20Prioritized%20AI%20Tile%20Structures))
  (bind _output_get (LocalVariables|SetNewLocalVar_0 (Utilities|Array|Get(acopy) NewParam)))
  (Utilities|Array|RemoveIndex NewParam)
  (return _output_get))

(fn AreTilesEqual
  (params (TileA :type AI%20Tile%20Structure) (TileB :type AI%20Tile%20Structure))
  (bind (_canpass _x _y) (Utilities|Struct|BreakAITile TileA))
  (bind (_canpass_2 _x_2 _y_2) (Utilities|Struct|BreakAITile TileB))
  (return (Math|Boolean|ANDBoolean (Math|Boolean|Equal(Boolean) _canpass _canpass_2) (== _x _x_2) (== _y _y_2))))

(fn MovementCost
  (params (From :type AI%20Tile%20Structure) (To :type AI%20Tile%20Structure))
  (if (.CanPass (Utilities|Struct|BreakAITile To))
    (return 1.0)
    (else
      (return 1e+03))))

(fn MoveinDirection
  (params (UnitDirection :type Vector) (DeltaTime :type Float%20%28single-precision%29))
  (bind _speed (Variables|Default|GetSpeed))
  (bind _returnvalue (* DeltaTime _speed))
  (bind _returnvalue_2 (* UnitDirection _returnvalue))
  (Transformation|SetActorLocation (+ (Transformation|GetActorLocation) _returnvalue_2) false false)
  (Math|Float|CompareFloat (.X (Math|Vector|BreakVector _returnvalue_2)) 0.0
    (:>
      (Transformation|SetActorRotation "0, 0, 0"))
    (:<
      (Transformation|SetActorRotation "0,180.000000, 0"))))

(fn PrintCosts
  (for (_ _array_index) (Variables|/Game/Blueprints/AI/AITileMap.AITileMap_C|GetMapTiles (Variables|Default|GetCurrentMap))
    (if (and (!= _array_index 0) (== (Math|Integer|%(Integer) _array_index (Variables|/Game/Blueprints/AI/AITileMap.AITileMap_C|GetMap%20Width (Variables|Default|GetCurrentMap))) 0))
      (Utilities|Array|Add (LocalVariables|GetLines) (LocalVariables|GetLine))
      (LocalVariables|SetLine ""))
    (if (== (.index (Variables|Default|GetCurrentTile)) _array_index)
      (LocalVariables|SetLine (Utilities|String|Append (LocalVariables|GetLine) "ME" " "))
      (elif (== _array_index (.index (Variables|Default|GetTargetTile)))
        (LocalVariables|SetLine (Utilities|String|Append (LocalVariables|GetLine) "TA" " "))
        (else
          (LocalVariables|SetLine (Utilities|String|Append (LocalVariables|GetLine) (Utilities|String|ToString(Float) (.Value (Utilities|Map|Find (Variables|Default|GetCostSoFar) _array_index))) " "))))))
  (Class|MyBlueprintFunctionLibrary|SaveStringArraytoFile (LocalVariables|GetLines)))

(fn TeleportOffscreen
  (bind _returnvalue (Math|Random|RandomFloatinRange -64.0 64.0))
  (bind _returnvalue_2 (Game|Player|GetPlayerPawn 0))
  (bind _returnvalue_3 (Transformation|GetActorLocation _returnvalue_2))
  (bind _returnvalue_4 (+ (.z _returnvalue_3) _returnvalue))
  (bind _asplayer_character (Utilities|Casting|CastToPlayerCharacter (Game|Player|GetPlayerPawn 0)))
  (if (Math|Random|RandomBool)
    (bind _returnvalue_5 (Default|GetCameraLeftBound _asplayer_character))
    (Transformation|SetActorLocation (Class|KismetMathLibrary|VectorBoundedtoBox (Math|Vector|MakeVector (- _returnvalue_5 3e+01) 0.0 _returnvalue_4) (Math|Vector|MakeVector 1e+01 0.0 (+ (+ (* (Variables|/Game/Blueprints/Character/PlayerCharacter.PlayerCharacter_C|GetMapZMax _asplayer_character) -1.0) (Variables|Default|GetZOffset)) 1e+01)) (Math|Vector|MakeVector (- (Variables|/Game/Blueprints/Character/PlayerCharacter.PlayerCharacter_C|GetMapXMax _asplayer_character) 1e+01) 0.0 (- (Variables|Default|GetZOffset) 1e+01))) false true)
    (else
      (bind _returnvalue_6 (Default|GetCameraRightBound _asplayer_character))
      (Transformation|SetActorLocation (Class|KismetMathLibrary|VectorBoundedtoBox (Math|Vector|MakeVector (+ _returnvalue_6 3e+01) 0.0 _returnvalue_4) (Math|Vector|MakeVector 1e+01 0.0 (+ (+ (* (Variables|/Game/Blueprints/Character/PlayerCharacter.PlayerCharacter_C|GetMapZMax _asplayer_character) -1.0) (Variables|Default|GetZOffset)) 1e+01)) (Math|Vector|MakeVector (- (Variables|/Game/Blueprints/Character/PlayerCharacter.PlayerCharacter_C|GetMapXMax _asplayer_character) 1e+01) 0.0 (- (Variables|Default|GetZOffset) 1e+01))) false true))))

(fn ChangeMaps
  (params (NewZOffset :type Float%20%28single-precision%29))
  (bind _output_get (Variables|Default|SetZOffset NewZOffset))
  (Math|Float|CompareFloat _output_get 0.0
    (:>
      (Variables|Default|SetCurrentMap (Variables|Default|GetFutureMap)))
    (:==
      (Variables|Default|SetCurrentMap (Variables|Default|GetPresentMap)))
    (:<
      (Variables|Default|SetCurrentMap (Variables|Default|GetPastMap))))
  (CallFunction|TeleportOffscreen)
  (bind _player (CallFunction|ASTar))
  (Variables|Default|SetLastKnownGoal _player))

(fn StopTrackingPlayer
  (Variables|Default|SetTrackingPlayer false))

(fn TakeDamage
  (params (Damage :type Float%20%28single-precision%29))
  (bind _output_get (Variables|Default|SetHP (- (Variables|Default|GetHP) Damage)))
  (if (<= _output_get 0.0)
    (CallFunction|Die)
    (else
      (CallFunction|DamageFlash))))

(fn Die
  (Game|SpawnActorfromClass "/Game/Blueprints/Misc/Explosion.Explosion_C" (Transformation|GetActorTransform) "Undefined" 0 0)
  (Variables|Default|SetTrackingPlayer false)
  (Variables|Default|SetRespawnTimer 1e+01)
  (Rendering|SetActorHiddenInGame true)
  (Collision|SetCollisionEnabled (Variables|Default|GetBox) "NoCollision")
  (CallFunction|SpawnItem))

(fn SpawnItem
  (bind _returnvalue (Transformation|GetActorTransform))
  (bind _output_get (LocalVariables|SetNum (Math|Random|RandomIntegerinRange 0 10)))
  (if (== (Math|Integer|%(Integer) _output_get 2) 0)
    (Game|SpawnActorfromClass "/Game/Blueprints/Pickups/Health.Health_C" _returnvalue "Undefined" 0 0)
    (elif (== (LocalVariables|GetNum) 3)
      (Game|SpawnActorfromClass "/Game/Blueprints/Pickups/SpreadShot.SpreadShot_C" _returnvalue "Undefined" 0 0))))

(fn Respawn
  (Variables|Default|SetHP (Variables|Default|GetMaxHP))
  (Rendering|SetActorHiddenInGame false)
  (Collision|SetCollisionEnabled (Variables|Default|GetBox) "QueryOnly")
  (Variables|Default|SetTrackingPlayer true)
  (CallFunction|TeleportOffscreen)
  (bind _player (CallFunction|ASTar))
  (Variables|Default|SetLastKnownGoal _player))