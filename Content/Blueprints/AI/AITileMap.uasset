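; Tile map actor that builds a coarse AI navigation grid from a Paper2D tile map, grouping tiles into square blocks.
; PopulateGrid stores each block as an AITile with passability, coordinates and indices of its four orthogonal neighbours.
; A block counts as solid when short Visibility traces at tile centres hit on more than half its tiles.
; GetTile maps a world position to its block, assuming 16-unit tiles on the XZ plane.
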(event EventBeginPlay)

(fn ConstructionScript)

(fn ConverttoCoordinates
  (params (Index :type Integer))
  (bind _map_width (Variables|Default|GetMap%20Width))
  (return (Math|Integer|%(Integer) Index _map_width) (/ Index _map_width)))

(fn ConverttoIndex
  (params (X :type Integer) (Y :type Integer))
  (bind _blockwidth (Variables|Default|GetBlockWidth))
  (return (+ (/ X _blockwidth) (* (/ Y _blockwidth) (/ (Variables|/Script/Paper2D.PaperTileMap|GetMapWidth (Variables|/Script/Paper2D.PaperTileMapComponent|GetTileMap (Variables|Default|GetRenderComponent))) _blockwidth)))))

(fn IsBlockSolid
  (params (TopLeftX :type Integer) (TopLeftY :type Integer))
  (bind _blockwidth (Variables|Default|GetBlockWidth))
  (bind _blockwidth_2 (Variables|Default|GetBlockWidth))
  (for _index (range 0 (- (* _blockwidth_2 _blockwidth_2) 1))
    (if (and (== (Math|Integer|%(Integer) _index _blockwidth_2) 0) (!= _index 0))
      (LocalVariables|SetLocalY (+ (LocalVariables|GetLocalY) 1))
      (LocalVariables|SetLocalX TopLeftX)
      (elif (not (!= _index 0))
        (LocalVariables|SetLocalX TopLeftX)
        (LocalVariables|SetLocalY TopLeftY)
        (else
          (LocalVariables|SetLocalX (+ (LocalVariables|GetLocalX) 1)))))
    (bind _output_get (LocalVariables|SetNewLocalVar_0 (Class|PaperTileMapComponent|GetTileCenterPosition (Variables|Default|GetRenderComponent) (LocalVariables|GetLocalX) (LocalVariables|GetLocalY) 0 true)))
    (bind _outhit (Collision|LineTraceByChannel _output_get (+ _output_get "0, 0,1.000000") "TraceTypeQuery1" false 0 "None" false))
    (if (.bBlockingHit (Collision|BreakHitResult _outhit))
      (LocalVariables|SetNumTilesSolid (+ (LocalVariables|GetNumTilesSolid) 1))))
  (return (> (LocalVariables|GetNumTilesSolid) (/ (* _blockwidth _blockwidth) 2))))

(fn GetTile
  (params (Position :type Vector))
  (bind _index (CallFunction|ConverttoIndex (Math|Float|Truncate (/ (.x Position) 16.0)) (Math|Float|Truncate (/ (.z Position) -16.0))))
  (return (Utilities|Array|Get(acopy) (Variables|Default|GetMapTiles) _index)))

(fn GetTileWorldPosition
  (params (MapX :type Integer) (MapY :type Integer))
  (bind _blockwidth (Variables|Default|GetBlockWidth))
  (bind _returnvalue (/ _blockwidth 2))
  (return (Class|PaperTileMapComponent|GetTileCenterPosition (Variables|Default|GetRenderComponent) (+ MapX _returnvalue) (+ MapY _returnvalue) 0 true)))

(fn PopulateGrid
  (bind _blockwidth (Variables|Default|GetBlockWidth))
  (bind _blockwidth_2 (Variables|Default|GetBlockWidth))
  (bind _rendercomponent (Variables|Default|GetRenderComponent))
  (bind _currentneighbours (Variables|Default|GetCurrentNeighbours))
  (bind _tilemap (Variables|/Script/Paper2D.PaperTileMapComponent|GetTileMap _rendercomponent))
  (bind _mapheight (Variables|/Script/Paper2D.PaperTileMap|GetMapHeight _tilemap))
  (bind _mapwidth (Variables|/Script/Paper2D.PaperTileMap|GetMapWidth _tilemap))
  (bind _returnvalue (* _mapwidth _mapheight))
  (Variables|Default|SetMap%20Width _mapwidth)
  (Utilities|Array|Resize (Variables|Default|GetMapTiles) (/ _returnvalue (* _blockwidth _blockwidth)))
  (for _index (range 0 (- _returnvalue (Variables|Default|GetBlockWidth)))
    (bind (_x _y) (CallFunction|ConverttoCoordinates _index))
    (bind _output_get (Variables|Default|SetCurrent%20X _x))
    (bind _output_get_2 (Variables|Default|SetCurrent%20Y _y))
    (if (and (== (Math|Integer|%(Integer) _output_get _blockwidth_2) 0) (== (Math|Integer|%(Integer) _output_get_2 _blockwidth_2) 0))
      (bind _index_2 (CallFunction|ConverttoIndex (Variables|Default|GetCurrent%20X) (Variables|Default|GetCurrent%20Y)))
      (Variables|Default|SetCurrentIndex _index_2)
      (Utilities|Array|Resize (Variables|Default|GetCurrentNeighbours) 0)
      ;[1 1 1] Populate Tile Grid
      (bind _is_solid (CallFunction|IsBlockSolid (Variables|Default|GetCurrent%20X) (Variables|Default|GetCurrent%20Y)))
      (Variables|Default|SetCurrentTileSolid _is_solid)
      ;[1 1 1] Top Center
      (if (> (Variables|Default|GetCurrent%20Y) 0)
        (bind _index_3 (CallFunction|ConverttoIndex (Variables|Default|GetCurrent%20X) (- (Variables|Default|GetCurrent%20Y) (Variables|Default|GetBlockWidth))))
        (if (Utilities|Array|IsValidIndex (Variables|Default|GetMapTiles) _index_3)
          (Utilities|Array|Add _currentneighbours _index_3)))
      ;[1 1 1] Bottom Center
      (if (< (Variables|Default|GetCurrent%20Y) (- (Variables|/Script/Paper2D.PaperTileMap|GetMapHeight (Variables|/Script/Paper2D.PaperTileMapComponent|GetTileMap (Variables|Default|GetRenderComponent))) (Variables|Default|GetBlockWidth)))
        (bind _index_4 (CallFunction|ConverttoIndex (Variables|Default|GetCurrent%20X) (+ (Variables|Default|GetCurrent%20Y) (Variables|Default|GetBlockWidth))))
        (if (Utilities|Array|IsValidIndex (Variables|Default|GetMapTiles) _index_4)
          (Utilities|Array|Add _currentneighbours _index_4)))
      ;[1 1 1] Left
      (if (> (Variables|Default|GetCurrent%20X) 0)
        (bind _index_5 (CallFunction|ConverttoIndex (- (Variables|Default|GetCurrent%20X) (Variables|Default|GetBlockWidth)) (Variables|Default|GetCurrent%20Y)))
        (if (Utilities|Array|IsValidIndex (Variables|Default|GetMapTiles) _index_5)
          (Utilities|Array|Add _currentneighbours _index_5)))
      ;[1 1 1] Right
      (if (< (Variables|Default|GetCurrent%20X) (- (Variables|Default|GetMap%20Width) 4))
        (bind _index_6 (CallFunction|ConverttoIndex (+ (Variables|Default|GetCurrent%20X) (Variables|Default|GetBlockWidth)) (Variables|Default|GetCurrent%20Y)))
        (if (Utilities|Array|IsValidIndex (Variables|Default|GetMapTiles) _index_6)
          (Utilities|Array|Add _currentneighbours _index_6)))
      (Utilities|Array|SetArrayElem (Variables|Default|GetMapTiles) (Variables|Default|GetCurrentIndex) (Utilities|Struct|MakeAITile (not (Variables|Default|GetCurrentTileSolid)) (Variables|Default|GetCurrent%20X) (Variables|Default|GetCurrent%20Y) (Variables|Default|GetCurrentIndex) _currentneighbours)))))