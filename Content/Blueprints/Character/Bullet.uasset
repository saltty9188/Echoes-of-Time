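; Bullet is a player-weapon style projectile that flies straight along its spawn facing at a set Speed, moved each Tick without sweep.
; Lifetime acts as an arming countdown, so Box overlaps count only after it reaches zero, and other Bullets are ignored for spreadshot.
; An armed hit destroys the bullet and uses a cast chain to deal fixed damage to Target or the AI, Future, Present and Past enemy types.
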(event OnComponentBeginOverlap(Box)
  (params (OverlappedComponent :type Primitive%20Component%20Object%20Reference) (OtherActor :type Actor%20Object%20Reference) (OtherComp :type Primitive%20Component%20Object%20Reference) (OtherBodyIndex :type Integer) (bFromSweep :type Boolean) (SweepResult :type Hit%20Result%20Structure%20%28by%20ref%29))
  ;[1 1 1] Ignore other bullets for spreadshot
  (bind _output_get (Variables|Default|SetHit%20Actor OtherActor))
  (Utilities|Casting|CastToBullet _output_get
    (:CastFailed
      ;[1 1 1] Don't fire on first frame
      (if (<= (Variables|Default|GetLifetime) 0.0)
        (Actor|DestroyActor)
        (Utilities|Casting|CastToNoTimeTravelZone (Variables|Default|GetHit%20Actor)
          (:then
            _)
          (:CastFailed
            _))
        (Utilities|Casting|CastToPlayerCharacter (Variables|Default|GetHit%20Actor)
          (:then
            _)
          (:CastFailed
            _))
        (Utilities|Casting|CastToHealth (Variables|Default|GetHit%20Actor)
          (:then
            _)
          (:CastFailed
            _))
        (Utilities|Casting|CastToSpreadShot (Variables|Default|GetHit%20Actor)
          (:then
            _)
          (:CastFailed
            _))
        ;[1 1 1] Deal damage
        (bind _asaienemy (Utilities|Casting|CastToAIEnemy (Variables|Default|GetHit%20Actor))
          (:then
            (Default|TakeDamage _asaienemy 15.0))
          (:CastFailed
            (bind _astarget (Utilities|Casting|CastToTarget (Variables|Default|GetHit%20Actor))
              (:then
                (Default|TakeDamage _astarget 1e+01))
              (:CastFailed
                (bind _asfuture_enemy (Utilities|Casting|CastToFutureEnemy (Variables|Default|GetHit%20Actor))
                  (:then
                    (Default|TakeDamage _asfuture_enemy 15.0))
                  (:CastFailed
                    (bind _aspresent_enemy (Utilities|Casting|CastToPresentEnemy (Variables|Default|GetHit%20Actor))
                      (:then
                        (Default|TakeDamage _aspresent_enemy 15.0))
                      (:CastFailed
                        (bind _aspast_enemy (Utilities|Casting|CastToPastEnemy (Variables|Default|GetHit%20Actor)))
                        (Default|TakeDamage _aspast_enemy 15.0)))))))))))))

(event EventBeginPlay
  ;[1 1 1] Set Facing Direction
  (Variables|Default|SetDirection (Math|Rotator|GetRotationXVector (Transformation|GetActorRotation))))

(event EventTick
  (params (DeltaSeconds :type Float%20%28single-precision%29))
  ;[1 1 1] Move The Bullet
  (Transformation|SetActorLocation (+ (* (Variables|Default|GetDirection) (* DeltaSeconds (Variables|Default|GetSpeed))) (Transformation|GetActorLocation)) false false)
  (if (> (Variables|Default|GetLifetime) 0.0)
    (Variables|Default|SetLifetime (- (Variables|Default|GetLifetime) DeltaSeconds))))

(fn ConstructionScript)