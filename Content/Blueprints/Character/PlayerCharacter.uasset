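; Player character for a side-scrolling 2D platformer shooter, with double jump, dash, spreadshot shooting and time travel between past and future.
; A State value drives flipbook animation, while Tick locks the Y axis, clamps the orthographic camera to map bounds and updates the HUD.
; Time travel shifts the player between map layers stacked in Z and notifies listeners through an event dispatcher.
; Damage grants invincibility frames; death fades out and respawns at the starting transform.
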(event Custom|On%20Death%20Anim%20Finish
  ;[1 1 1] Death Animation and Respawn
  (Actor|DestroyActor (stale Custom|OnDeath _outactor))
  (Transformation|SetActorTransform (Variables|Default|GetSpawn) false true)
  (Variables|Default|SetHP (Variables|Default|GetMaxHP))
  (Variables|Default|SetTimer 0.0)
  (bind _output_get (Variables|Default|SetCurrentZOffset 0.0))
  (Default|CallTimeTravelEventDispatcher _output_get)
  ;;[1 1 1] Teleport
  (Audio|PlaySound2D "/Game/Sounds/teleport.teleport" 1.0 1.0 0.0 0 0)
  (bind _returnvalue (Game|SpawnActorfromClass "/Game/Blueprints/Misc/TeleportEffect.TeleportEffect_C" (Math|Transform|MakeTransform "0,1.000000, 0" "0, 0, 0" "2.000000,1,2.000000") "Undefined" 0 0))
  (Components|Timeline|SetPlayRate (Variables|/Game/Blueprints/Misc/TeleportEffect.TeleportEffect_C|GetPaperFlipbook _returnvalue) 0.4)
  (Transformation|AttachActorToActor _returnvalue (Game|Player|GetPlayerPawn 0) "None" "KeepRelative" "KeepRelative" "KeepRelative" true)
  (bind (_outactor _returnvalue_2) (Sequencer|Player|CreateLevelSequencePlayer "/Game/LevelSequences/FadeInDeath.FadeInDeath"))
  (Sequencer|Player|Play _returnvalue_2 :!class /Script/MovieScene.MovieSceneSequencePlayer)
  (EventDispatchers|AssignOnFinished _returnvalue_2 (delegate Custom|OnFinished_Event_0))
  (Input|EnableInput (Game|GetPlayerController 0))
  (Variables|Default|SetState "NewEnumerator3")
  (Default|CallDeathEventDispatcher))

(event Custom|OnDeath
  (params (PitDeath :type Boolean))
  ;[1 1 1] Death Animation and Respawn
  (bind (_outactor _returnvalue) (Sequencer|Player|CreateLevelSequencePlayer "/Game/LevelSequences/FadeOutDeath.FadeOutDeath"))
  (EventDispatchers|BindEventtoOnFinished _returnvalue (delegate Custom|On%20Death%20Anim%20Finish))
  (Sequencer|Player|Play _returnvalue :!class /Script/MovieScene.MovieSceneSequencePlayer)
  (Audio|PlaySound2D "/Game/Sounds/Player_Death.Player_Death" 1.0 1.0 0.0 0 0)
  ;;[1 1 1] Disable input and lock X position
  (Character|LaunchCharacter "0, 0,-1.000000" true true)
  (Input|DisableInput (Game|GetPlayerController 0))
  (bind _outactors (Actor|GetAllActorsOfClass "/Game/Blueprints/AI/AIEnemy.AIEnemy_C"))
  (for _array_element _outactors
    (Default|StopTrackingPlayer _array_element)))

(event Custom|OnFinished_Event_0
  ;[1 1 1] Death Animation and Respawn
  (Actor|DestroyActor (stale Custom|On%20Death%20Anim%20Finish _outactor)))

(event Custom|UpdateAnimtation
  (bind _sprite (Variables|Default|GetSprite))
  ;[1 1 1] Update Animation
  (if (and (Math|Float|NearlyEqual(Float) (Math|Float|Absolute(Float) (Math|Vector|VectorLength (Transformation|GetVelocity))) 0.0 1e-06) (Utilities|Enum|NotEqual(Enum) (Variables|Default|GetState) "NewEnumerator4"))
    (Variables|Default|SetState "NewEnumerator3"))
  (switch Utilities|FlowControl|Switch|SwitchonPlayerStates (Variables|Default|GetState)
    (:NewEnumerator0
      (Sprite|SetFlipbook _sprite "/Game/Sprites/Characters/Run/PlayerRun.PlayerRun")
      (Components|Timeline|SetLooping _sprite true)
      (Audio|Components|Audio|Play _sprite))
    (:NewEnumerator1
      (Utilities|FlowControl|Sequence
        (:then_0
          (if (Variables|Default|GetJustJumped)
            (Sprite|SetFlipbook _sprite "/Game/Sprites/Characters/Jump/PlayerJump.PlayerJump")
            (Components|Timeline|PlayfromStart _sprite)
            (Variables|Default|SetJustJumped false)))
        (:then_1
          (Sprite|SetFlipbook _sprite "/Game/Sprites/Characters/Jump/PlayerJump.PlayerJump")
          (Components|Timeline|SetLooping _sprite false))))
    (:NewEnumerator2
      (Sprite|SetFlipbook _sprite "/Game/Sprites/Characters/Dash/PlayerDash1.PlayerDash1")
      (Components|Timeline|SetLooping _sprite true)
      (Audio|Components|Audio|Play _sprite))
    (:NewEnumerator3
      (Sprite|SetFlipbook _sprite "/Game/Sprites/Characters/Idle/Idle.Idle")
      (Components|Timeline|SetLooping _sprite true)
      (Audio|Components|Audio|Play _sprite))
    (:NewEnumerator4
      (Utilities|FlowControl|Sequence
        (:then_0
          (if (Variables|Default|GetJustDied)
            (Sprite|SetFlipbook _sprite "/Game/Sprites/Characters/Death/PlayerDeath.PlayerDeath")
            (Components|Timeline|PlayfromStart _sprite)
            (Variables|Default|SetJustDied false)))
        (:then_1
          (Sprite|SetFlipbook _sprite "/Game/Sprites/Characters/Death/PlayerDeath.PlayerDeath")
          (Components|Timeline|SetLooping _sprite false))))))

(event Custom|DamageFlash
  (bind _sprite (Variables|Default|GetSprite))
  ;[1 1 1] Flicker For Damage Flash
  (Utilities|ForLoopwithDelay 0 9 0.2
    (:Loop%20Body
      (Rendering|SetVisibility _sprite (not (Rendering|IsVisible _sprite)) false))))

(event EventTick
  (params (DeltaSeconds :type Float%20%28single-precision%29))
  (bind _returnvalue (Transformation|GetActorLocation))
  (bind (_x _y _z) (Math|Vector|BreakVector _returnvalue))
  ;[1 1 1] Constrain Player Y Location
  (Transformation|SetActorLocation (Math|Vector|MakeVector _x -1e+01 _z) false true)
  (CallFunction|ConstrainCamera)
  (CallFunction|UpdateHUD)
  (CallFunction|UpdateAnimtation)
  (if (> (Variables|Default|GetIFrameTimer) 0.0)
    (Variables|Default|SetIFrameTimer (- (Variables|Default|GetIFrameTimer) DeltaSeconds))))

(event EventBeginPlay
  ;[1 1 1] Set Respawn Point
  (Variables|Default|SetSpawn (Transformation|GetActorTransform))
  (bind _returnvalue (UserInterface|CreateWidget "/Game/Blueprints/UI/HUDWidget.HUDWidget_C"))
  (bind _output_get (Variables|Default|SetHUDReference _returnvalue))
  (UserInterface|Viewport|AddtoViewport _output_get 0))

(event EventOnLanded
  (params (Hit :type Hit%20Result%20Structure%20%28by%20ref%29))
  ;[1 1 1] Jump/DoubleJump
  (Variables|Default|SetJumpNumber 0)
  (if (Utilities|Enum|NotEqual(Enum) (Variables|Default|GetState) "NewEnumerator4")
    (Variables|Default|SetState "NewEnumerator3")))

(event Input|ActionEvents|InputActionSprint
  (params (Key :type Key%20Structure :default "None"))
  (bind _returnvalue (Transformation|GetVelocity))
  ;[1 1 1] Dashing
  (:Pressed
    (if (Math|Vector|NotEqual(Vector) _returnvalue "0, 0, 0" 0.0001)
      (Math|Float|CompareFloat (stale Input|AxisEvents|InputAxisLeftRight AxisValue) 0.0
        (:>
          (Variables|Default|SetIsMovingRight true)
          (Character|LaunchCharacter (+ _returnvalue "700.000000, 0, 0") true true))
        (:<
          (Variables|Default|SetIsMovingRight false)
          (Character|LaunchCharacter (+ _returnvalue "-800.000000, 0, 0") true true)))
      (Variables|Default|SetState "NewEnumerator2")
      (Utilities|FlowControl|Delay 0.2)
      (Character|LaunchCharacter (select (Variables|Default|GetIsMovingRight) "300.000000, 0, 0" "-300.000000, 0, 0") true false))))

(event Input|ActionEvents|InputActionShoot
  (params (Key :type Key%20Structure :default "None"))
  (bind _ismovingright (Variables|Default|GetIsMovingRight))
  (bind _ismovingright_2 (Variables|Default|GetIsMovingRight))
  (bind _ismovingright_3 (Variables|Default|GetIsMovingRight))
  (:Pressed
    ;[1 1 1] Shooting
    (if (Utilities|Enum|NotEqual(Enum) (Variables|Default|GetState) "NewEnumerator2")
      (Audio|PlaySound2D "/Game/Sounds/8bit_gunloop_explosion.8bit_gunloop_explosion" 1.0 1.0 0.0 0 0)
      (Game|SpawnActorfromClass "/Game/Blueprints/Character/Bullet.Bullet_C" (Math|Transform|MakeTransform (+ (Transformation|GetWorldLocation (Variables|Default|GetSprite)) (Math|Vector|SelectVector "15.000000,0.000000,5.000000" "-15.000000,1.000000,5.000000" _ismovingright_2)) (select _ismovingright_2 "0, 0, 0" "0,180.000000, 0")) "Undefined" 0 0)
      (if (Variables|Default|GetHasSpreadshot)
        (Game|SpawnActorfromClass "/Game/Blueprints/Character/Bullet.Bullet_C" (Math|Transform|MakeTransform (+ (Transformation|GetWorldLocation (Variables|Default|GetSprite)) (Math|Vector|SelectVector "15.000000,0.000000,5.000000" "-15.000000,1.000000,5.000000" _ismovingright_3)) (select _ismovingright_3 "10.000000, 0,0.000000" "10.000000,180.000000,0.000000")) "Undefined" 0 0)
        (Game|SpawnActorfromClass "/Game/Blueprints/Character/Bullet.Bullet_C" (Math|Transform|MakeTransform (+ (Transformation|GetWorldLocation (Variables|Default|GetSprite)) (Math|Vector|SelectVector "15.000000,0.000000,5.000000" "-15.000000,1.000000,5.000000" _ismovingright)) (select _ismovingright "-10.000000, 0,0.000000" "-10.000000,180.000000,0.000000")) "Undefined" 0 0)))))

(event Input|ActionEvents|InputActionJump
  (params (Key :type Key%20Structure :default "None"))
  ;[1 1 1] Jump/DoubleJump
  (:Pressed
    (if (< (Variables|Default|GetJumpNumber) 2)
      (Variables|Default|SetState "NewEnumerator1")
      (Variables|Default|SetJustJumped true)
      (Character|LaunchCharacter (+ (Transformation|GetVelocity) "0, 0,400.000000") true true)
      (Math|Integer|IncrementInt (Variables|Default|GetJumpNumber)))))

(event Input|ActionEvents|InputActionPause
  (params (Key :type Key%20Structure :default "None"))
  (bind _returnvalue (Game|GetPlayerController 0))
  ;[1 1 1] Pause Game
  (:Pressed
    (Utilities|IsValid (Variables|Default|GetPauseMenuReference)
      (:Is%20Valid
        _)
      (:Is%20Not%20Valid
        (bind _returnvalue_2 (UserInterface|CreateWidget "/Game/Blueprints/UI/PauseMenu.PauseMenu_C"))
        (Variables|Default|SetPauseMenuReference _returnvalue_2)))
    (Variables|/Script/Engine.PlayerController|SetbShowMouseCursor _returnvalue true)
    (Input|SetInputModeUIOnly _returnvalue (Variables|Default|GetPauseMenuReference) "DoNotLock")
    (UserInterface|Viewport|AddtoViewport (Variables|Default|GetPauseMenuReference) 0)
    (Game|SetGamePaused true)))

(event Input|AxisEvents|InputAxisLeftRight
  (params (AxisValue :type Float%20%28single-precision%29))
  (bind _sprite (Variables|Default|GetSprite))
  ;[1 1 1] Movement
  (Math|Float|CompareFloat AxisValue 0.0
    (:>
      (Variables|Default|SetIsMovingRight true)
      (Transformation|SetWorldRotation _sprite "0, 0, 0" false false))
    (:<
      (Variables|Default|SetIsMovingRight false)
      (Transformation|SetWorldRotation _sprite "0,180.000000, 0" false false)))
  (Pawn|Input|AddMovementInput "1.000000, 0, 0" AxisValue true)
  (if (not (or (Utilities|Enum|Equal(Enum) (Variables|Default|GetState) "NewEnumerator2") (Utilities|Enum|Equal(Enum) (Variables|Default|GetState) "NewEnumerator1")))
    (Variables|Default|SetState "NewEnumerator0")))

(event Input|KeyboardEvents|E
  (params (Key :type Key%20Structure :default "None"))
  ;[1 1 1] Time Travel
  (:Pressed
    (bind _returnvalue (CallFunction|CanGoFuture))
    (if _returnvalue
      (CallFunction|Teleport)
      (Utilities|FlowControl|Delay 0.2)
      (CallFunction|GoFuture))))

(event Input|KeyboardEvents|Q
  (params (Key :type Key%20Structure :default "None"))
  ;[1 1 1] Time Travel
  (:Pressed
    (bind _returnvalue (CallFunction|CanGoPast))
    (if _returnvalue
      (CallFunction|Teleport)
      (Utilities|FlowControl|Delay 0.2)
      (CallFunction|GoPast))))

(fn ConstructionScript)

(fn Dash
  (Pawn|Input|AddMovementInput "0, 0, 0" (* (Input|AxisValues|GetLeftRight) 2.0) false))

(fn StopDash
  (Pawn|Input|AddMovementInput "0, 0, 0" (Input|AxisValues|GetLeftRight) false))

(fn GetCameraLeftBound
  (bind _camera (Variables|Default|GetCamera))
  (return (- (.X (Math|Vector|BreakVector (Transformation|GetWorldLocation _camera))) (/ (Variables|/Script/Engine.CameraComponent|GetOrthoWidth _camera) 2.0))))

(fn GetCameraRightBound
  (bind _camera (Variables|Default|GetCamera))
  (return (+ (/ (Variables|/Script/Engine.CameraComponent|GetOrthoWidth _camera) 2.0) (.X (Math|Vector|BreakVector (Transformation|GetWorldLocation _camera))))))

(fn ConstrainCamera
  (bind _returnvalue (Transformation|GetActorLocation))
  (bind _camera (Variables|Default|GetCamera))
  (bind _camera_2 (Variables|Default|GetCamera))
  (bind _camera_3 (Variables|Default|GetCamera))
  (bind _currentzoffset (Variables|Default|GetCurrentZOffset))
  (bind _mapxmax (Variables|Default|GetMapXMax))
  (bind _camera_4 (Variables|Default|GetCamera))
  (bind _camera_5 (Variables|Default|GetCamera))
  (bind _currentzoffset_2 (Variables|Default|GetCurrentZOffset))
  (bind _mapzmax (Variables|Default|GetMapZMax))
  (bind _returnvalue_2 (Transformation|GetWorldLocation _camera))
  (bind _returnvalue_3 (Transformation|GetWorldLocation _camera_4))
  (bind (_x _y _z) (Math|Vector|BreakVector _returnvalue))
  (bind _returnvalue_4 (- _currentzoffset_2 _mapzmax))
  (bind _returnvalue_5 (Transformation|GetWorldLocation _camera_2))
  (bind _returnvalue_6 (Transformation|GetWorldLocation _camera_3))
  (bind (_x_2 _y_2) (Math|Vector|BreakVector _returnvalue_3))
  (bind (_x_3 _y_3 _z_2) (Math|Vector|BreakVector _returnvalue_2))
  (bind (_x_4 _y_4) (Math|Vector|BreakVector _returnvalue_5))
  (bind (_x_5 _y_5 _z_3) (Math|Vector|BreakVector _returnvalue_6))
  ;[1 1 1] Follow Player
  (Transformation|SetWorldLocation _camera_5 (Math|Vector|MakeVector _x (.Y (Math|Vector|BreakVector (Transformation|GetWorldLocation _camera_5))) _z) false false)
  ;[1 1 1] Check Right Side
  (bind _returnvalue_7 (CallFunction|GetCameraRightBound))
  (if (>= _returnvalue_7 _mapxmax)
    (Transformation|SetWorldLocation _camera (Math|Vector|MakeVector (- _mapxmax (/ (Variables|/Script/Engine.CameraComponent|GetOrthoWidth _camera) 2.0)) _y_3 _z_2) false true)
    (else
      ;[1 1 1] Check Right Side
      (bind _returnvalue_8 (CallFunction|GetCameraLeftBound))
      (if (<= _returnvalue_8 0.0)
        (Transformation|SetWorldLocation _camera_3 (Math|Vector|MakeVector (/ (Variables|/Script/Engine.CameraComponent|GetOrthoWidth _camera_3) 2.0) _y_5 _z_3) false true))))
  ;[1 1 1] Check Top Side
  (bind _returnvalue_9 (CallFunction|GetCameraTopBound))
  (bind _returnvalue_10 (CallFunction|GetHalfCameraHeight))
  (if (>= _returnvalue_9 _currentzoffset)
    (Transformation|SetWorldLocation _camera_4 (Math|Vector|MakeVector _x_2 _y_2 (- _currentzoffset _returnvalue_10)) false true)
    (else
      ;[1 1 1] Check Bottom Side
      (bind _returnvalue_11 (CallFunction|GetCameraBottomBound))
      (bind _returnvalue_12 (CallFunction|GetHalfCameraHeight))
      (if (<= _returnvalue_11 _returnvalue_4)
        (Transformation|SetWorldLocation _camera_2 (Math|Vector|MakeVector _x_4 _y_4 (+ _returnvalue_4 _returnvalue_12)) false true)))))

(fn GetHalfCameraHeight
  (bind _camera (Variables|Default|GetCamera))
  (return (/ (/ (Variables|/Script/Engine.CameraComponent|GetOrthoWidth _camera) (Variables|/Script/Engine.CameraComponent|GetAspectRatio _camera)) 2.0)))

(fn GetCameraTopBound
  (bind _returnvalue (CallFunction|GetHalfCameraHeight))
  (return (+ _returnvalue (.Z (Math|Vector|BreakVector (Transformation|GetWorldLocation (Variables|Default|GetCamera)))))))

(fn GetCameraBottomBound
  (bind _returnvalue (CallFunction|GetHalfCameraHeight))
  (return (- (.Z (Math|Vector|BreakVector (Transformation|GetWorldLocation (Variables|Default|GetCamera)))) _returnvalue)))

(fn GoFuture
  (Variables|Default|SetCurrentZOffset (+ (Variables|Default|GetCurrentZOffset) 3e+03))
  (bind _asplayer_character (Utilities|Casting|CastToPlayerCharacter (Game|Player|GetPlayerPawn 0)))
  (Transformation|SetActorLocation _asplayer_character (Math|Vector|MakeVector (.X (Math|Vector|BreakVector (Transformation|GetActorLocation _asplayer_character))) (.Y (Math|Vector|BreakVector (Transformation|GetActorLocation _asplayer_character))) (+ (.Z (Math|Vector|BreakVector (Transformation|GetActorLocation _asplayer_character))) 3e+03)) false true)
  (Default|CallTimeTravelEventDispatcher (Variables|Default|GetCurrentZOffset)))

(fn GoPast
  (Variables|Default|SetCurrentZOffset (- (Variables|Default|GetCurrentZOffset) 3e+03))
  (bind _asplayer_character (Utilities|Casting|CastToPlayerCharacter (Game|Player|GetPlayerPawn 0)))
  (Transformation|SetActorLocation _asplayer_character (Math|Vector|MakeVector (.X (Math|Vector|BreakVector (Transformation|GetActorLocation _asplayer_character))) (.Y (Math|Vector|BreakVector (Transformation|GetActorLocation _asplayer_character))) (- (.Z (Math|Vector|BreakVector (Transformation|GetActorLocation _asplayer_character))) 3e+03)) false true)
  (Default|CallTimeTravelEventDispatcher (Variables|Default|GetCurrentZOffset)))

(fn Teleport
  (Audio|PlaySound2D "/Game/Sounds/172206__fins__teleport.172206__fins__teleport" 1.0 1.0 0.0 0 0)
  (bind _returnvalue (Game|SpawnActorfromClass "/Game/Blueprints/Misc/TeleportEffect.TeleportEffect_C" (Math|Transform|MakeTransform "0, 0, 0") "Undefined" 0 0))
  (Transformation|AttachActorToActor _returnvalue self "None" "KeepRelative" "KeepRelative" "KeepWorld" true)
  (return))

(fn CanGoFuture
  (return (and (Variables|Default|GetCanTimeTravel) (not (>= (Variables|Default|GetCurrentZOffset) 3e+03)))))

(fn CanGoPast
  (return (and (Variables|Default|GetCanTimeTravel) (not (<= (Variables|Default|GetCurrentZOffset) -3e+03)))))

(fn UpdateHUD
  (bind _hp (Variables|Default|GetHP))
  (bind _returnvalue (CallFunction|CanGoFuture))
  (bind _returnvalue_2 (CallFunction|CanGoPast))
  (Default|UpdateHUD (Variables|Default|GetHUDReference) _hp (/ _hp (Variables|Default|GetMaxHP)) _returnvalue _returnvalue_2 (Variables|Default|GetTimer)))

(fn TakeDamage
  (params (Damage :type Float%20%28single-precision%29))
  (if (<= (Variables|Default|GetIFrameTimer) 0.0)
    (Variables|Default|SetHP (- (Variables|Default|GetHP) Damage))
    (Variables|Default|SetIFrameTimer 2.0)
    (if (> (Variables|Default|GetHP) 0.0)
      (Audio|PlaySound2D "/Game/Sounds/Hit.Hit" 0.7 1.0 0.0 0 0)
      (Variables|Default|SetHasSpreadshot false)
      (CallFunction|DamageFlash)
      (else
        (Variables|Default|SetState "NewEnumerator4")
        (Variables|Default|SetJustDied true)
        (CallFunction|OnDeath false)))))

(fn ReceiveHealth
  (params (NewHealth :type Float%20%28single-precision%29))
  (bind _maxhp (Variables|Default|GetMaxHP))
  (bind _output_get (Variables|Default|SetHP (+ (Variables|Default|GetHP) NewHealth)))
  (if (> _output_get _maxhp)
    (Variables|Default|SetHP _maxhp)))