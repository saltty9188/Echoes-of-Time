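; 2D caveman enemy that patrols along X between its start point and a set distance, flipping at each end.
; Tick moves it and swaps to an attack flipbook near the player, while overlapping the player deals damage.
; Hits flash the sprite, and death spawns an explosion, a possible health or spread-shot drop, then hides it without collision.
; The player's death dispatcher resets it at its spawn with full HP.
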(event Custom|DamageFlash
  (bind _paperflipbook (Variables|Default|GetPaperFlipbook))
  ;[1 1 1] Damage Flash
  (Utilities|ForLoopwithDelay 0 1 0.1
    (:Loop%20Body
      (Rendering|SetVisibility _paperflipbook (not (Rendering|IsVisible _paperflipbook)) false))
    (:Completed
      (Rendering|SetVisibility (Variables|Default|GetPaperFlipbook) true false))))

(event Custom|RespawnEvent
  (CallFunction|Respawn))

(event EventBeginPlay
  (bind _returnvalue (Transformation|GetActorLocation))
  (Variables|Default|SetRunPoints (Utilities|Array|MakeArray _returnvalue (+ _returnvalue (Math|Vector|MakeVector (Variables|Default|GetDistance) 0.0 0.0))))
  (Variables|Default|SetSpawn (Transformation|GetActorTransform))
  (bind _asplayer_character (Utilities|Casting|CastToPlayerCharacter (Game|Player|GetPlayerPawn 0)))
  (EventDispatchers|BindEventtoDeathEventDispatcher _asplayer_character (delegate Custom|RespawnEvent)))

(event Collision|EventActorBeginOverlap
  (params (OtherActor :type Actor%20Object%20Reference))
  (bind _asplayer_character (Utilities|Casting|CastToPlayerCharacter OtherActor))
  (Default|TakeDamage _asplayer_character 15.0))

(event EventTick
  (params (DeltaSeconds :type Float%20%28single-precision%29))
  (bind _returnvalue (Transformation|GetActorLocation))
  (bind _paperflipbook (Variables|Default|GetPaperFlipbook))
  ;[1 1 1] Move and flip enemy
  (if (Variables|Default|GetFacingRight)
    (Transformation|SetActorRotation "0, 0, 0")
    (Transformation|SetActorLocation (+ (Transformation|GetActorLocation) (* "1.000000, 0, 0" (* (Variables|Default|GetSpeed) DeltaSeconds))) false false)
    (Variables|Default|SetFacingRight (not (< (Math|Vector|Distance(Vector) (Utilities|Array|Get(acopy) (Variables|Default|GetRunPoints) 1) _returnvalue) 1.0)))
    (else
      (Transformation|SetActorRotation "0,180.000000, 0")
      (Transformation|SetActorLocation (+ (Transformation|GetActorLocation) (* "-1.000000, 0, 0" (* DeltaSeconds (Variables|Default|GetSpeed)))) false false)
      (Variables|Default|SetFacingRight (< (Math|Vector|Distance(Vector) _returnvalue (Utilities|Array|Get(acopy) (Variables|Default|GetRunPoints))) 1.0))))
  ;[1 1 1] Set attacking flipbook when close to player
  (if (<= (Math|Vector|Distance(Vector) (Transformation|GetActorLocation) (Transformation|GetActorLocation (Game|Player|GetPlayerPawn 0))) (Variables|Default|GetRange))
    (Sprite|SetFlipbook _paperflipbook "/Game/Sprites/Enemies/Caveman/Run/caveman_attack.caveman_attack")
    (Utilities|String|Reverse _paperflipbook)
    (else
      (Sprite|SetFlipbook _paperflipbook "/Game/Sprites/Enemies/Caveman/Attack/caveman_Run.caveman_Run"))))

(fn ConstructionScript)

(fn TakeDamage
  (params (Damage :type Float%20%28single-precision%29))
  (bind _output_get (Variables|Default|SetHP (- (Variables|Default|GetHP) Damage)))
  (if (<= _output_get 0.0)
    (CallFunction|Die)
    (else
      (CallFunction|DamageFlash))))

(fn Respawn
  (Variables|Default|SetHP (Variables|Default|GetMaxHP))
  (Rendering|SetActorHiddenInGame false)
  (Collision|SetCollisionEnabled (Variables|Default|GetBox) "QueryOnly")
  (Transformation|SetActorTransform (Variables|Default|GetSpawn)))

(fn Die
  (Game|SpawnActorfromClass "/Game/Blueprints/Misc/Explosion.Explosion_C" (Transformation|GetActorTransform) "Undefined" 0 0)
  (Rendering|SetActorHiddenInGame true)
  (Collision|SetCollisionEnabled (Variables|Default|GetBox) "NoCollision")
  (CallFunction|SpawnItem))

(fn SpawnItem
  (bind _returnvalue (Transformation|GetActorTransform))
  (bind _returnvalue_2 (Math|Transform|MakeTransform (.location _returnvalue) (.rotation _returnvalue)))
  (bind _output_get (LocalVariables|SetNum (Math|Random|RandomIntegerinRange 0 10)))
  (if (== (Math|Integer|%(Integer) _output_get 2) 0)
    (Game|SpawnActorfromClass "/Game/Blueprints/Pickups/Health.Health_C" _returnvalue_2 "Undefined" 0 0)
    (elif (== (LocalVariables|GetNum) 3)
      (Game|SpawnActorfromClass "/Game/Blueprints/Pickups/SpreadShot.SpreadShot_C" _returnvalue_2 "Undefined" 0 0))))