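; Target is a damageable enemy actor that explodes when its health runs out.
; TakeDamage subtracts from Health and calls Die at zero or below, which spawns an Explosion, hides the actor and disables RenderComponent collision instead of destroying it.
; A separate DamageFlash event blinks the actor by toggling its hidden state in a short delayed loop, but nothing in this Blueprint calls it.
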(event Custom|DamageFlash
  ;[1 1 1] Damage Flash
  (Utilities|ForLoopwithDelay 0 1 0.1
    (:Loop%20Body
      (Rendering|SetActorHiddenInGame (not (Variables|Rendering|GetbHidden))))))

(event EventBeginPlay)

(event Collision|EventActorBeginOverlap
  (params (OtherActor :type Actor%20Object%20Reference)))

(event EventTick
  (params (DeltaSeconds :type Float%20%28single-precision%29)))

(fn ConstructionScript)

(fn TakeDamage
  (params (Damage :type Float%20%28single-precision%29))
  (bind _output_get (Variables|Default|SetHealth (- (Variables|Default|GetHealth) Damage)))
  (if (<= _output_get 0.0)
    (CallFunction|Die)))

(fn Die
  (Game|SpawnActorfromClass "/Game/Blueprints/Misc/Explosion.Explosion_C" (Transformation|GetActorTransform) "Undefined" 0 0)
  (Rendering|SetActorHiddenInGame true)
  (Collision|SetCollisionEnabled (Variables|Default|GetRenderComponent) "NoCollision"))