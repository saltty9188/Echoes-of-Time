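; NextLevel is a level exit trigger that moves the player to the level set in its Level variable.
; When a PaperCharacter overlaps its Box, every AIEnemy stops tracking the player and a slowed TeleportEffect attaches to the character with a whoosh sound.
; It disables the character's input, hides its RenderComponent and plays the FadeOut sequence to fade to white, opening the level when that sequence finishes.
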(event OnComponentBeginOverlap(Box)
  (params (OverlappedComponent :type Primitive%20Component%20Object%20Reference) (OtherActor :type Actor%20Object%20Reference) (OtherComp :type Primitive%20Component%20Object%20Reference) (OtherBodyIndex :type Integer) (bFromSweep :type Boolean) (SweepResult :type Hit%20Result%20Structure%20%28by%20ref%29))
  (bind _aspaper_character (Utilities|Casting|CastToPaperCharacter OtherActor))
  (bind _outactors (Actor|GetAllActorsOfClass "/Game/Blueprints/AI/AIEnemy.AIEnemy_C"))
  (for _array_element _outactors
    (Variables|/Game/Blueprints/AI/AIEnemy.AIEnemy_C|SetTrackingPlayer _array_element false))
  ;[1 1 1] Create teleport effect
  (Audio|PlaySound2D "/Game/Sounds/whoosh__phaser_.whoosh__phaser_" 1.0 1.0 0.0 0 0)
  (bind _returnvalue (Game|SpawnActorfromClass "/Game/Blueprints/Misc/TeleportEffect.TeleportEffect_C" (Math|Transform|MakeTransform "0, 0, 0" "0, 0, 0" "2.000000,1,2.000000") "Undefined" 0 0))
  (Components|Timeline|SetPlayRate (Variables|/Game/Blueprints/Misc/TeleportEffect.TeleportEffect_C|GetPaperFlipbook _returnvalue) 0.4)
  ;[1 1 1] Fade to white
  (Transformation|AttachActorToActor _returnvalue _aspaper_character "None" "KeepRelative" "KeepRelative" "KeepWorld" true)
  (bind _returnvalue_2 (Sequencer|Player|CreateLevelSequencePlayer "/Game/LevelSequences/FadeOut.FadeOut"))
  (EventDispatchers|AssignOnFinished _returnvalue_2 (delegate Custom|OnFinished_Event_0))
  (Sequencer|Player|Play _returnvalue_2 :!class /Script/MovieScene.MovieSceneSequencePlayer)
  (Input|DisableInput _aspaper_character 0)
  (Rendering|SetVisibility (Variables|Default|GetRenderComponent) false false))

(event Custom|OnFinished_Event_0
  ;[1 1 1] Fade to white
  (Game|OpenLevel(byObjectReference) (Variables|Components|GetLevel) false))

(fn ConstructionScript)