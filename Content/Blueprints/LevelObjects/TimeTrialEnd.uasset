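; Time trial finish trigger that ends a run, judges the player's time and returns to the Main level.
; On box overlap it disables player input, compares the timer to the saved best for Level1 or otherwise Level2, and saves new records.
; Records show confetti and fanfare, misses play failure music, each with a HUD message and music pause.
; When the jingle ends, music resumes and a teleport effect and fade-out sequence precede the level load.
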(event OnComponentBeginOverlap(Box)
  (params (OverlappedComponent :type Primitive%20Component%20Object%20Reference) (OtherActor :type Actor%20Object%20Reference) (OtherComp :type Primitive%20Component%20Object%20Reference) (OtherBodyIndex :type Integer) (bFromSweep :type Boolean) (SweepResult :type Hit%20Result%20Structure%20%28by%20ref%29))
  (bind _time_trial_save (Variables|Default|GetTime%20Trial%20Save))
  (bind _asplayer_character (Utilities|Casting|CastToPlayerCharacter OtherActor))
  (Input|DisableInput _asplayer_character (Game|GetPlayerController 0))
  (bind _returnvalue (Game|GetCurrentLevelName true))
  (if (Utilities|Enum|Equal(Enum) _returnvalue "Level1")
    (if (<= (Variables|/Game/Blueprints/Character/PlayerCharacter.PlayerCharacter_C|GetTimer _asplayer_character) (Variables|/Game/Blueprints/TimeTrialSave.TimeTrialSave_C|GetLevel1BestTime _time_trial_save))
      ;[1 1 1] Save Best Time
      (Variables|/Game/Blueprints/TimeTrialSave.TimeTrialSave_C|SetLevel1BestTime _time_trial_save (Variables|/Game/Blueprints/Character/PlayerCharacter.PlayerCharacter_C|GetTimer _asplayer_character))
      (SaveGame|SaveGametoSlot _time_trial_save "Save")
      ;[1 1 1] Victory Music
      (Rendering|SetVisibility (Variables|Default|GetConfetti) true true :!label _label)
      (bind _returnvalue_2 (Audio|SpawnSound2D "/Game/Music/Fanfare_03__1_.Fanfare_03__1_" 1.0 1.0 0.0 0))
      (EventDispatchers|BindEventtoOnAudioFinished _returnvalue_2 (delegate Custom|OnFanfareEnd))
      (bind _asplayer_character_2 (Utilities|Casting|CastToPlayerCharacter (Game|Player|GetPlayerPawn 0)))
      (Default|NewRecord (Variables|/Game/Blueprints/Character/PlayerCharacter.PlayerCharacter_C|GetHUDReference _asplayer_character_2))
      (Default|CallPauseMusicDispatch)
      (else
        ;[1 1 1] Failure Music
        (bind _returnvalue_3 (Audio|SpawnSound2D "/Game/Music/Icy_Game_Over.Icy_Game_Over" 1.0 1.0 0.0 0 :!label _label_2))
        (EventDispatchers|BindEventtoOnAudioFinished _returnvalue_3 (delegate Custom|OnFanfareEnd))
        (bind _asplayer_character_3 (Utilities|Casting|CastToPlayerCharacter (Game|Player|GetPlayerPawn 0)))
        (Default|TryAgain (Variables|/Game/Blueprints/Character/PlayerCharacter.PlayerCharacter_C|GetHUDReference _asplayer_character_3))
        (Default|CallPauseMusicDispatch)))
    (elif (<= (Variables|/Game/Blueprints/Character/PlayerCharacter.PlayerCharacter_C|GetTimer _asplayer_character) (Variables|/Game/Blueprints/TimeTrialSave.TimeTrialSave_C|GetLevel2BestTime _time_trial_save))
      (Variables|/Game/Blueprints/TimeTrialSave.TimeTrialSave_C|SetLevel2BestTime _time_trial_save (Variables|/Game/Blueprints/Character/PlayerCharacter.PlayerCharacter_C|GetTimer _asplayer_character))
      (SaveGame|SaveGametoSlot _time_trial_save "Save")
      (goto _label)
      (else
        (goto _label_2)))))

(event Custom|OnFinished_Event_0
  ;[1 1 1] Fade to white
  (Game|OpenLevel(byObjectReference) "/Game/Levels/Main.Main"))

(event Custom|OnFanfareEnd
  (Default|CallResumeMusicDispatch)
  ;[1 1 1] Create teleport effect
  (Audio|PlaySound2D "/Game/Sounds/whoosh__phaser_.whoosh__phaser_" 1.0 1.0 0.0 0 0)
  (bind _returnvalue (Game|SpawnActorfromClass "/Game/Blueprints/Misc/TeleportEffect.TeleportEffect_C" (Math|Transform|MakeTransform "0, 0, 0" "0, 0, 0" "2.000000,1,2.000000") "Undefined" 0 0))
  (Components|Timeline|SetPlayRate (Variables|/Game/Blueprints/Misc/TeleportEffect.TeleportEffect_C|GetPaperFlipbook _returnvalue) 0.4)
  ;[1 1 1] Fade to white
  (Transformation|AttachActorToActor _returnvalue (Game|Player|GetPlayerPawn 0) "None" "KeepRelative" "KeepRelative" "KeepWorld" true)
  (bind _returnvalue_2 (Sequencer|Player|CreateLevelSequencePlayer "/Game/LevelSequences/FadeOut.FadeOut"))
  (EventDispatchers|AssignOnFinished _returnvalue_2 (delegate Custom|OnFinished_Event_0))
  (Sequencer|Player|Play _returnvalue_2 :!class /Script/MovieScene.MovieSceneSequencePlayer))

(event EventBeginPlay
  (bind _returnvalue (SaveGame|LoadGamefromSlot "Save"))
  (bind _astime_trial_save (Utilities|Casting|CastToTimeTrialSave _returnvalue))
  (Variables|Default|SetTime%20Trial%20Save _astime_trial_save)
  (Rendering|SetVisibility (Variables|Default|GetConfetti) false true))

(event Collision|EventActorBeginOverlap
  (params (OtherActor :type Actor%20Object%20Reference)))

(event EventTick
  (params (DeltaSeconds :type Float%20%28single-precision%29)))

(fn ConstructionScript)