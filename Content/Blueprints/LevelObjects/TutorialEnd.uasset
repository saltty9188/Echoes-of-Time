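; Trigger actor that ends the tutorial and sends the player to Level1 when a PaperCharacter overlaps its box.
; The overlap disables the box and player input, then a delayed loop spawns a few explosions at random points around the actor.
; It then plays a whoosh, attaches a slowed teleport effect to the character and hides its RenderComponent.
; A FadeOut level sequence runs, and its finished event opens Level1.
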(event OnComponentBeginOverlap(Box)
  (params (OverlappedComponent :type Primitive%20Component%20Object%20Reference) (OtherActor :type Actor%20Object%20Reference) (OtherComp :type Primitive%20Component%20Object%20Reference) (OtherBodyIndex :type Integer) (bFromSweep :type Boolean) (SweepResult :type Hit%20Result%20Structure%20%28by%20ref%29))
  (bind _aspaper_character (Utilities|Casting|CastToPaperCharacter OtherActor))
  (Collision|SetCollisionEnabled (Variables|Default|GetBox) "NoCollision")
  (Input|DisableInput _aspaper_character (Game|GetPlayerController 0))
  (Utilities|ForLoopwithDelay 0 3 0.3
    (:Loop%20Body
      (Game|SpawnActorfromClass "/Game/Blueprints/Misc/Explosion.Explosion_C" (Math|Transform|MakeTransform (Math|Random|RandomPointinBoundingBox (Transformation|GetActorLocation) "16.000000, 0,16.000000")) "Undefined" 0 0))
    (:Completed
      ;[1 1 1] Create teleport effect
      (Audio|PlaySound2D "/Game/Sounds/whoosh__phaser_.whoosh__phaser_" 1.0 1.0 0.0 0 0)
      (bind _returnvalue (Game|SpawnActorfromClass "/Game/Blueprints/Misc/TeleportEffect.TeleportEffect_C" (Math|Transform|MakeTransform "0,1.000000, 0" "0, 0, 0" "2.000000,1,2.000000") "Undefined" 0 0))
      (Components|Timeline|SetPlayRate (Variables|/Game/Blueprints/Misc/TeleportEffect.TeleportEffect_C|GetPaperFlipbook _returnvalue) 0.4)
      (Transformation|AttachActorToActor _returnvalue _aspaper_character "None" "KeepRelative" "KeepRelative" "KeepWorld" true)
      ;[1 1 1] Fade to white
      (bind _returnvalue_2 (Sequencer|Player|CreateLevelSequencePlayer "/Game/LevelSequences/FadeOut.FadeOut"))
      (EventDispatchers|AssignOnFinished _returnvalue_2 (delegate Custom|OnFinished_Event_0))
      (Sequencer|Player|Play _returnvalue_2 :!class /Script/MovieScene.MovieSceneSequencePlayer)
      (Rendering|SetVisibility (Variables|Default|GetRenderComponent) false false))))

(event Custom|OnFinished_Event_0
  ;[1 1 1] Fade to white
  (Game|OpenLevel(byObjectReference) "/Game/Levels/Level1.Level1" false))

(event EventBeginPlay)

(event Collision|EventActorBeginOverlap
  (params (OtherActor :type Actor%20Object%20Reference)))

(event EventTick
  (params (DeltaSeconds :type Float%20%28single-precision%29)))

(fn ConstructionScript)

(fn SpawnExplosions
  (params (NumExplosions :type Integer)))